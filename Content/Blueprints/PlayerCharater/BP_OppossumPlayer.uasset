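; Player character Blueprint for the opossum, handling shooting, dashing, movement direction and damage from chicken characters.
; Shoot press and release drive a BP_Launcher found among child actors by FindThing, with recoil applied on press.
; Tick combines movement inputs into a Direction vector, Left Shift dashes, and hits from BP_ChickenCharacter call Hurt.
; The 0 key destroys the player and shows the WH_GameOver widget with UI-only input.
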(event EventBeginPlay)

(event Collision|EventActorBeginOverlap
  (params (OtherActor :type Actor%20Object%20Reference)))

(event EventTick
  (params (DeltaSeconds :type Float%20%28single-precision%29))
  (Variables|Default|SetDirection (Math|Vector2D|MakeVector2D (+ (Input|AxisValues|GetMoveForward) (Input|AxisValues|GetMoveBackwards)) (+ (Input|AxisValues|GetMoveRight) (Input|AxisValues|GetMoveLeft)))))

(event Collision|EventHit
  (params (MyComp :type Primitive%20Component%20Object%20Reference) (Other :type Actor%20Object%20Reference) (OtherComp :type Primitive%20Component%20Object%20Reference) (bSelfMoved :type Boolean) (HitLocation :type Vector :default "0, 0, 0") (HitNormal :type Vector :default "0, 0, 0") (NormalImpulse :type Vector :default "0, 0, 0") (Hit :type Hit%20Result%20Structure%20%28by%20ref%29))
  (Utilities|Casting|CastToBP_ChickenCharacter Other)
  (Class|CPPOppossumPlayer|Hurt 10))

(event Input|ActionEvents|InputActionShoot
  (params (Key :type Key%20Structure :default "None"))
  (bind _childactors (Actor|GetAllChildActors true))
  (:Pressed
    (bind _newparam1 (CallFunction|FindThing _childactors))
    (bind _asbp_launcher (Utilities|Casting|CastToBP_Launcher _newparam1))
    (Default|Down _asbp_launcher)
    (Class|CPPOppossumPlayer|ApplyRecoil -5e+02))
  (:Released
    (bind _newparam1_2 (CallFunction|FindThing _childactors))
    (bind _asbp_launcher_2 (Utilities|Casting|CastToBP_Launcher _newparam1_2))
    (Default|Release _asbp_launcher_2)))

(event Input|KeyboardEvents|0
  (params (Key :type Key%20Structure :default "None"))
  (:Pressed
    (Actor|DestroyActor)
    (bind _returnvalue (UserInterface|CreateWidget "/Game/UI/WH_GameOver.WH_GameOver_C"))
    (UserInterface|Viewport|AddtoViewport _returnvalue 0)
    (Input|SetInputModeUIOnly 0 0 "DoNotLock" false)))

(event Input|KeyboardEvents|LeftShift
  (params (Key :type Key%20Structure :default "None"))
  (:Pressed
    (Class|CPPOppossumPlayer|Dash)))

(fn ConstructionScript)

(fn FindThing
  (params (NewParam :type Array%20of%20Actor%20Object%20References))
  (for _array_element NewParam
    (bind _asbp_launcher (Utilities|Casting|CastToBP_Launcher _array_element))
    (return _asbp_launcher)))