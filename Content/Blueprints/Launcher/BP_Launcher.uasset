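; BP_Launcher is a launcher that fires BP_Bullet projectiles from its parent actor, expected to be BP_OppossumPlayer.
; Down and Release events track button and firing state, and every Release calls Fire.
; Fire spawns a bullet above the parent and applies a fixed-strength, upward-arcing impulse along the player's Direction, printing the horizontal vector.
; Charge and reload logic is disconnected from Tick, so charge never affects the shot.
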(event Custom|Release
  (Variables|Default|SetFiring false)
  (Variables|Default|SetButtonDown false)
  (CallFunction|Fire))

(event Custom|Down
  ;[1 1 1] Check if it can fire
  (if (<= (stale _output_get) 0.0)
    (Variables|Default|SetFiring true)
    (else
      (Variables|Default|SetButtonDown true))))

(event EventTick
  (params (DeltaSeconds :type Float%20%28single-precision%29)))

(event Collision|EventActorBeginOverlap
  (params (OtherActor :type Actor%20Object%20Reference)))

(fn ConstructionScript)

(fn Fire
  (bind _returnvalue (Game|SpawnActorfromClass "/Game/Blueprints/Launcher/Bullet/BP_Bullet.BP_Bullet_C" (Math|Conversions|ToTransform(Vector) (Math|Transform|TransformLocation (Transformation|GetWorldTransform (Variables|/Script/Engine.Actor|GetRootComponent (Actor|GetParentActor))) "0.000000,0.000000,200.000000")) "Undefined" "MultiplyWithRoot" 0 0))
  (bind _asbp_oppossum_player (Utilities|Casting|CastToBP_OppossumPlayer (Actor|GetParentActor)))
  (Physics|AddImpulse (Variables|/Game/Blueprints/Launcher/Bullet/BP_Bullet.BP_Bullet_C|GetSphere _returnvalue) (Math|Conversions|ToVector(Vector2D) (* (Variables|/Game/Blueprints/PlayerCharater/BP_OppossumPlayer.BP_OppossumPlayer_C|GetDirection _asbp_oppossum_player) "(X=20000.000000,Y=20000.000000)") 1e+04) "None" false)
  (Development|PrintString (Utilities|String|ToString(Vector2d) (* (Variables|/Game/Blueprints/PlayerCharater/BP_OppossumPlayer.BP_OppossumPlayer_C|GetDirection _asbp_oppossum_player) "(X=20000.000000,Y=20000.000000)"))))