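; BP_ChickenCharacter is an AI chicken character that pursues the opossum player and bursts into feathers when shot.
; It spawns its default controller on BeginPlay, then PawnSensing triggers an AI move toward a seen player.
; CanSeeEnemy turns true on sighting and clears through a retriggerable delay once sightings stop.
; Bullet hits spawn hit or death feather effects depending on Health, which this graph never changes.
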(event OnSeePawn(PawnSensing)
  (params (Pawn :type Pawn%20Object%20Reference))
  ;[1 1 1] AI Targeting
  (bind _ascpp_oppossum_player (Utilities|Casting|CastToCPP_OppossumPlayer Pawn))
  (Utilities|FlowControl|Sequence
    (:then_0
      (Variables|Default|SetCan%20See%20Enemy true)
      (AI|AIMoveTo self "0, 0, 0" _ascpp_oppossum_player 5.0 false
        (:then
          (Utilities|FlowControl|DoOnce false))))
    (:then_1
      (Utilities|FlowControl|RetriggerableDelay 0.2)
      (Variables|Default|SetCan%20See%20Enemy false))))

(event EventBeginPlay
  (Pawn|SpawnDefaultController))

(event Collision|EventActorBeginOverlap
  (params (OtherActor :type Actor%20Object%20Reference)))

(event Collision|EventHit
  (params (MyComp :type Primitive%20Component%20Object%20Reference) (Other :type Actor%20Object%20Reference) (OtherComp :type Primitive%20Component%20Object%20Reference) (bSelfMoved :type Boolean) (HitLocation :type Vector :default "0, 0, 0") (HitNormal :type Vector :default "0, 0, 0") (NormalImpulse :type Vector :default "0, 0, 0") (Hit :type Hit%20Result%20Structure%20%28by%20ref%29))
  ;[1 1 1] Spawn Particle Effects at Chicken Loaction
  (Utilities|Casting|CastToBP_Bullet Other)
  (Variables|Default|SetHit%20Location HitLocation)
  (if (> (Variables|Default|Gethealth) 0)
    (Niagara|SpawnSystematLocation "/Game/Materials/Materials/NS_Feathers.NS_Feathers" (Variables|Default|GetHit%20Location) "0, 0, 0" "1.500000,1.500000,1.500000")
    (Development|PrintString "HIT")
    (else
      (Niagara|SpawnSystematLocation "/Game/Materials/Materials/NS_DeathFeathers.NS_DeathFeathers" (Variables|Default|GetHit%20Location) "0, 0, 0" "1.500000,1.500000,1.500000")
      (Development|PrintString "Death"))))

(fn ConstructionScript)