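; Chicken enemy pawn that moves toward the opossum player on sight and reacts to hits with feather effects.
; PawnSensing drives AIMoveTo and sets CanSeeEnemy, which a retriggerable delay clears shortly after the last sighting.
; Hits from non-chickens store the location, call Hurt and spawn normal or death feathers based on Damage; destruction spawns steam there.
; Box component hits apply a fixed velocity-change impulse along Y to the box.
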(event OnSeePawn(PawnSensing)
  (params (Pawn :type Pawn%20Object%20Reference))
  ;[1 1 1] AI Targeting
  (bind _ascpp_oppossum_player (Utilities|Casting|CastToCPP_OppossumPlayer Pawn))
  (Utilities|FlowControl|Sequence
    (:then_0
      (Variables|Default|SetCan%20See%20Enemy true)
      (AI|AIMoveTo self "0, 0, 0" _ascpp_oppossum_player 5.0 false
        (:then
          (Utilities|FlowControl|DoOnce false))))
    (:then_1
      (Utilities|FlowControl|RetriggerableDelay 0.2)
      (Variables|Default|SetCan%20See%20Enemy false))))

(event OnComponentHit(Box)
  (params (HitComponent :type Primitive%20Component%20Object%20Reference) (OtherActor :type Actor%20Object%20Reference) (OtherComp :type Primitive%20Component%20Object%20Reference) (NormalImpulse :type Vector :default "0, 0, 0") (Hit :type Hit%20Result%20Structure%20%28by%20ref%29))
  (Physics|AddImpulse (Variables|Default|GetBox) "0.000000,200.000000,0.000000" "None" true))

(event Collision|EventHit
  (params (MyComp :type Primitive%20Component%20Object%20Reference) (Other :type Actor%20Object%20Reference) (OtherComp :type Primitive%20Component%20Object%20Reference) (bSelfMoved :type Boolean) (HitLocation :type Vector :default "0, 0, 0") (HitNormal :type Vector :default "0, 0, 0") (NormalImpulse :type Vector :default "0, 0, 0") (Hit :type Hit%20Result%20Structure%20%28by%20ref%29))
  (bind _damage (Variables|Default|GetDamage))
  ;[1 1 1] Spawn Particle Effects at Chicken Loaction
  (Utilities|Casting|CastToBP_Chicken Other
    (:CastFailed
      (Variables|Default|SetHit%20Location HitLocation)
      (Class|CPChicken|Hurt _damage)
      (if (> _damage 0)
        (Niagara|SpawnSystematLocation "/Game/Materials/Materials/NS_Feathers.NS_Feathers" (Variables|Default|GetHit%20Location) "0, 0, 0" "1.500000,1.500000,1.500000")
        (Development|PrintString "HIT")
        (else
          (Niagara|SpawnSystematLocation "/Game/Materials/Materials/NS_DeathFeathers.NS_DeathFeathers" (Variables|Default|GetHit%20Location) "0, 0, 0" "1.500000,1.500000,1.500000")
          (Development|PrintString "Death"))))))

(event EventDestroyed
  ;[1 1 1] Spawn Particle Effects at Chicken Loaction
  (Effects|SpawnEmitteratLocation "/Game/StarterContent/Particles/P_Steam_Lit.P_Steam_Lit" (Variables|Default|GetHit%20Location)))

(fn ConstructionScript)